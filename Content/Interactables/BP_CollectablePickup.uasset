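; BP_CollectablePickup is an interactable physics pickup, built around a RadioAsset component, that the player can carry and drop.
; Through interact, it checks and sets the player's IsHolding flag, disables physics and collision, then snaps RadioAsset to the player's Arrow1, keeping relative rotation.
; Drop calls DetachFromActor on the actor rather than the attached component, then restores collision and physics without clearing IsHolding.
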(event EventBeginPlay)

(event Collision|EventActorBeginOverlap
  (params (OtherActor :type Actor%20Object%20Reference)))

(event EventTick
  (params (DeltaSeconds :type Float%20%28single-precision%29)))

(event EventINTInteract
  (params (Player%20Ref :type BP%20Player%20Char%20Object%20Reference))
  (bind _radioasset (Variables|Default|GetRadioAsset))
  (if (not (Variables|/Game/Player/BP_PlayerChar.BP_PlayerChar_C|GetIsHolding? Player%20Ref))
    (Variables|/Game/Player/BP_PlayerChar.BP_PlayerChar_C|SetIsHolding? Player%20Ref true)
    (Physics|SetSimulatePhysics _radioasset false)
    (Collision|SetCollisionEnabled _radioasset "NoCollision")
    (Transformation|AttachComponentToComponent (Variables|Default|GetRadioAsset) (Variables|/Game/Player/BP_PlayerChar.BP_PlayerChar_C|GetArrow1 Player%20Ref) "None" "SnapToTarget" "KeepRelative" "KeepRelative" true)))

(event EventINTDrop
  (bind _radioasset (Variables|Default|GetRadioAsset))
  (Transformation|DetachFromActor "KeepWorld" "KeepWorld" "KeepWorld")
  (Collision|SetCollisionEnabled _radioasset "QueryAndPhysics")
  (Physics|SetSimulatePhysics _radioasset true))

(fn ConstructionScript)